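; Underwater zone actor that shifts a referenced directional light's intensity and color between default and underwater looks.
; Two collision volumes, open water and cave, share one IsUnderwater flag, set before the BP_TestCharacter cast so any overlapping actor toggles it.
; Tick interpolates intensity and a blend alpha at TransitionSpeed.
; Color lerps from its current value by that alpha, which falls toward zero on exit.
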(event OnComponentBeginOverlap(Collision_Underwater)
  (params (OverlappedComponent :type Primitive%20Component%20Object%20Reference) (OtherActor :type Actor%20Object%20Reference) (OtherComp :type Primitive%20Component%20Object%20Reference) (OtherBodyIndex :type Integer) (bFromSweep :type Boolean) (SweepResult :type Hit%20Result%20Structure%20%28by%20ref%29))
  ;[0.3229 1 0.998] Underwater
  (Variables|Default|SetIsUnderwater true)
  (Utilities|Casting|CastToBP_TestCharacter OtherActor))

(event OnComponentEndOverlap(Collision_Underwater)
  (params (OverlappedComponent :type Primitive%20Component%20Object%20Reference) (OtherActor :type Actor%20Object%20Reference) (OtherComp :type Primitive%20Component%20Object%20Reference) (OtherBodyIndex :type Integer))
  ;[1 0.9556 0.4492] Ground
  (Variables|Default|SetIsUnderwater false)
  (Utilities|Casting|CastToBP_TestCharacter OtherActor))

(event OnComponentBeginOverlap(Collision_UnderwaterCave)
  (params (OverlappedComponent :type Primitive%20Component%20Object%20Reference) (OtherActor :type Actor%20Object%20Reference) (OtherComp :type Primitive%20Component%20Object%20Reference) (OtherBodyIndex :type Integer) (bFromSweep :type Boolean) (SweepResult :type Hit%20Result%20Structure%20%28by%20ref%29))
  ;[0.3229 1 0.998] Underwater
  (Variables|Default|SetIsUnderwater true)
  (Utilities|Casting|CastToBP_TestCharacter OtherActor))

(event OnComponentEndOverlap(Collision_UnderwaterCave)
  (params (OverlappedComponent :type Primitive%20Component%20Object%20Reference) (OtherActor :type Actor%20Object%20Reference) (OtherComp :type Primitive%20Component%20Object%20Reference) (OtherBodyIndex :type Integer))
  ;[1 0.9556 0.4492] Ground
  (Variables|Default|SetIsUnderwater false)
  (Utilities|Casting|CastToBP_TestCharacter OtherActor))

(event EventTick
  (params (DeltaSeconds :type Float%20%28single-precision%29))
  (bind _isunderwater (Variables|Default|GetIsUnderwater))
  ;[1 1 1] Intensity
  (bind _output_get (Variables|Default|SetCurrentLightIntensity (Math|Interpolation|FInterpTo (Variables|Default|GetCurrentLightIntensity) (select _isunderwater (Variables|Default|GetUnderwaterIntensity) (Variables|Default|GetDefaultIntensity)) DeltaSeconds (Variables|Default|GetTransitionSpeed))))
  (bind _output_get_2 (Variables|Default|SetDirectionalLightRef (Variables|Default|GetDirectionalLightRef)))
  (Rendering|Components|Light|SetIntensity (Variables|/Script/Engine.Light|GetLightComponent _output_get_2) _output_get)
  ;[0.598 0.6675 1] Color
  (bind _output_get_3 (Variables|Default|SetCurrentAlpha (Math|Interpolation|FInterpTo (Variables|Default|GetCurrentAlpha) (select _isunderwater 1.0 0.0) DeltaSeconds (Variables|Default|GetTransitionSpeed))))
  (bind _output_get_4 (Variables|Default|SetCurrentLightColor (Math|Color|Lerp(LinearColor) (Variables|Default|GetCurrentLightColor) (select (Variables|Default|GetIsUnderwater) (Variables|Default|GetUnderwaterColor) (Variables|Default|GetDefaultColor)) _output_get_3)))
  (Rendering|Components|Light|SetLightColor (Variables|/Script/Engine.Light|GetLightComponent _output_get_2) _output_get_4 true))

(fn ConstructionScript)