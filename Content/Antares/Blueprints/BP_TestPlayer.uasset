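; Test player Blueprint that publishes the player's world position to materials.
; Each Tick writes the location of player character 0, rather than its own, into the PlayerPosition vector of the MCP_PlayerPosition parameter collection.
; An unconnected branch that would toggle IsFlying from the actor's height and print fly or walk never runs.
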(event EventBeginPlay)

(event Collision|EventActorBeginOverlap
  (params (OtherActor :type Actor%20Object%20Reference)))

(event EventTick
  (params (DeltaSeconds :type Float%20%28single-precision%29))
  (Rendering|Material|SetVectorParameterValue "/Game/Antares/Materials/SafeZone/MCP_PlayerPosition.MCP_PlayerPosition" "PlayerPosition" (Math|Conversions|ToLinearColor(Vector) (Transformation|GetActorLocation (Game|GetPlayerCharacter 0))) :!class /Script/Engine.KismetMaterialLibrary))

(fn ConstructionScript)