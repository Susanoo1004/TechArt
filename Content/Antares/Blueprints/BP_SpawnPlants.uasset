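; Actor that grows BP_Plants on nearby surfaces tagged "SpawnPlants" as it moves.
; Each moving tick advances a timer whose delay comes from a runtime curve sampled by current speed.
; When it elapses, line traces along twelve directions built in the construction script find tagged surfaces.
; Randomly spread traces around those directions then spawn and initialize a random number of plants, rotated from the impact normal.
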(event EventTick
  (params (DeltaSeconds :type Float%20%28single-precision%29))
  (bind _returnvalue (Transformation|GetActorLocation))
  (bind _returnvalue_2 (Transformation|GetActorLocation))
  (bind _spreadradius (Variables|Properties|GetSpreadRadius))
  (bind _goodimpacts (Variables|Properties|GetGoodImpacts))
  (Utilities|SpawnDelaybySpeed DeltaSeconds)
  (if (not (Utilities|Operators|EqualEqual (Transformation|GetActorLocation) (Variables|Properties|GetLastPos) 0.0))
    (Variables|Properties|SetLastPos (Transformation|GetActorLocation))
    (bind _output_get (Variables|Properties|SetElapsedTimeSpawnDelay (+ DeltaSeconds (Variables|Properties|GetElapsedTimeSpawnDelay))))
    (if (>= _output_get (Variables|Properties|GetSpawnDelay))
      (Variables|Properties|SetElapsedTimeSpawnDelay (- (Variables|Properties|GetElapsedTimeSpawnDelay) (Variables|Properties|GetSpawnDelay)))
      (Utilities|Array|Clear (Variables|Properties|GetGoodImpacts))
      (for _array_element (Variables|Properties|GetDirections)
        (bind (_outhit _returnvalue_3) (Collision|LineTraceByChannel _returnvalue (+ _returnvalue (* _array_element (Variables|Properties|GetDetectionRadius))) "TraceTypeQuery1" false 0 "None"))
        (if _returnvalue_3
          (if (Actor|ActorHasTag (.HitActor (Collision|BreakHitResult _outhit)) "SpawnPlants")
            (Utilities|Array|Add (Variables|Properties|GetGoodImpacts) _array_element))))
      (if (not (Utilities|Array|IsEmpty _goodimpacts))
        (for _array_element_2 _goodimpacts
          (for _index (range 0 (Math|Random|RandomIntegerinRange (Variables|Properties|GetSpawn%20min) (Variables|Properties|GetSpawn%20max)))
            (bind (_outhit_2 _returnvalue_4) (Collision|LineTraceByChannel _returnvalue_2 (+ _returnvalue_2 (* (Variables|Properties|GetDetectionRadius) (Math|Vector|MakeVector (* (.x _array_element_2) (Math|Trig|Cos(Radians) (Math|Random|RandomFloatinRange 0.0 _spreadradius))) (* (.y _array_element_2) (Math|Trig|Sin(Radians) (Math|Random|RandomFloatinRange 0.0 _spreadradius))) (.z _array_element_2)))) "TraceTypeQuery1" false 0 "None"))
            (if _returnvalue_4
              (bind _returnvalue_5 (Game|SpawnActorfromClass "/Game/Antares/Blueprints/BP_Plants.BP_Plants_C" (Math|Transform|MakeTransform (.location _outhit_2) (Math|Conversions|RotationFromXVector (+ (.impactnormal _outhit_2) "0.000000,90.000000,0.000000"))) "Undefined" "MultiplyWithRoot" 0 0))
              (Default|InitializePlant _returnvalue_5))))))))

(event EventBeginPlay
  (Variables|Properties|SetLastPos (Transformation|GetActorLocation)))

(fn ConstructionScript
  (CallFunction|GetDirections))

(fn ScanFloor
  (Class|KismetSystemLibrary|DrawDebugConeinDegrees (Transformation|GetActorLocation) (* (Transformation|GetActorUpVector) -1.0) 5e+02 3e+01 3e+01 12 "(R=1.000000,G=1.000000,B=1.000000,A=1.000000)" 0.0 0.0))

(fn GetDirections
  (Variables|Properties|SetDirections (Utilities|Array|MakeArray "1.000000,0.000000,0.000000" "-1.000000,0.000000,0.000000" "0.000000,1.000000,0.000000" "0.000000,-1.000000,0.000000" "0.000000,0.000000,1.000000" "0.000000,0.000000,-1.000000" "1.000000,1.000000,1.000000" "-1.000000,-1.000000,-1.000000" "1.000000,-1.000000,1.000000" "-1.000000,1.000000,-1.000000" "1.000000,1.000000,-1.000000" "-1.000000,-1.000000,1.000000")))