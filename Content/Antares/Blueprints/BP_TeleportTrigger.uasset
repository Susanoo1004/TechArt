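; BP_TeleportTrigger is a box trigger that moves BP_TestCharacter to a TargetPoint behind a screen fade.
; On box overlap it creates a TransitionWidget, plays its FadeIn, and after a delay sets the character's location to the TargetPoint.
; It then plays FadeOut and removes the widget after a second delay.
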(event OnComponentBeginOverlap(Box)
  (params (OverlappedComponent :type Primitive%20Component%20Object%20Reference) (OtherActor :type Actor%20Object%20Reference) (OtherComp :type Primitive%20Component%20Object%20Reference) (OtherBodyIndex :type Integer) (bFromSweep :type Boolean) (SweepResult :type Hit%20Result%20Structure%20%28by%20ref%29))
  (bind _asbp_test_character (Utilities|Casting|CastToBP_TestCharacter OtherActor))
  (bind _returnvalue (UserInterface|CreateWidget "/Game/Antares/UI/TransitionWidget.TransitionWidget_C"))
  (UserInterface|Viewport|AddtoViewport _returnvalue 0)
  (UserInterface|Animation|PlayAnimation _returnvalue (Variables|/Game/Antares/UI/TransitionWidget.TransitionWidget_C|GetFadeIn _returnvalue) 0.0 1 "Forward" 1.0 false)
  (Utilities|FlowControl|Delay 2.0)
  (Transformation|SetActorLocation _asbp_test_character (Transformation|GetActorLocation (Variables|Default|GetTargetPoint)) false false)
  (UserInterface|Animation|PlayAnimation _returnvalue (Variables|/Game/Antares/UI/TransitionWidget.TransitionWidget_C|GetFadeOut _returnvalue) 0.0 1 "Forward" 1.0 false)
  (Utilities|FlowControl|Delay 2.0)
  (Widget|RemovefromParent _returnvalue))

(event EventBeginPlay)

(event Collision|EventActorBeginOverlap
  (params (OtherActor :type Actor%20Object%20Reference)))

(event EventTick
  (params (DeltaSeconds :type Float%20%28single-precision%29)))

(fn ConstructionScript)