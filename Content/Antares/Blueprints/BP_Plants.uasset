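; Short-lived plant actor that appears as a random mesh, changes scale over its lifetime, then destroys itself.
; InitializePlant, not called within this Blueprint, picks a random PlantsList index and plays the PlantLife timeline.
; Each timeline update reapplies the chosen mesh and sets its scale from the GrowthAndFade track.
; VisibilityOff and WhichPlant, which toggle component visibility, are never run and look like leftovers.
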(event Custom|InitializePlant
  (Variables|Default|SetRandomPlantIndex (Math|Random|RandomIntegerinRange 0 (- (Utilities|Array|Length (Variables|Default|GetPlantsList)) 1)))
  (bind _growth_and_fade (Timeline|PlantLife PlayFromStart)
    (:Update
      (Components|StaticMesh|SetStaticMesh (Variables|Default|GetPlant) (Utilities|Array|Get(acopy) (Variables|Default|GetPlantsList) (Variables|Default|GetRandomPlantIndex)))
      (Transformation|SetRelativeScale3D (Variables|Default|GetPlant) (Math|Conversions|ToVector(Float) _growth_and_fade)))
    (:Finished
      (Actor|DestroyActor))))

(event EventBeginPlay)

(event Collision|EventActorBeginOverlap
  (params (OtherActor :type Actor%20Object%20Reference)))

(event EventTick
  (params (DeltaSeconds :type Float%20%28single-precision%29)))

(fn ConstructionScript)