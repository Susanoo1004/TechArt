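; BP_SafeZone is a safe zone actor that tracks whether the player is inside its SafeZone sphere component.
; On BeginPlay it caches the BP_TestCharacter instance as Player.
; The sphere's begin and end overlap events set the PlayerInside flag for that actor only.
; The file only maintains the flag, with no protective effect of its own, and Tick is empty.
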(event OnComponentBeginOverlap(SafeZone)
  (params (OverlappedComponent :type Primitive%20Component%20Object%20Reference) (OtherActor :type Actor%20Object%20Reference) (OtherComp :type Primitive%20Component%20Object%20Reference) (OtherBodyIndex :type Integer) (bFromSweep :type Boolean) (SweepResult :type Hit%20Result%20Structure%20%28by%20ref%29))
  (if (== OtherActor (Variables|Default|GetPlayer))
    (Variables|Default|SetPlayerInside true)))

(event OnComponentEndOverlap(SafeZone)
  (params (OverlappedComponent :type Primitive%20Component%20Object%20Reference) (OtherActor :type Actor%20Object%20Reference) (OtherComp :type Primitive%20Component%20Object%20Reference) (OtherBodyIndex :type Integer))
  (if (== OtherActor (Variables|Default|GetPlayer))
    (Variables|Default|SetPlayerInside false)))

(event EventBeginPlay
  (bind _returnvalue (Actor|GetActorOfClass "/Game/Antares/Blueprints/BP_TestCharacter.BP_TestCharacter_C"))
  (Variables|Default|SetPlayer _returnvalue))

(event EventTick
  (params (DeltaSeconds :type Float%20%28single-precision%29)))

(fn ConstructionScript)