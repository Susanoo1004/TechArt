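; BP_TestCharacter is a test character that publishes the player's location to materials and toggles a flying state by height.
; Each Tick writes player 0's location into the PlayerPosition vector of the MCP_PlayerPosition parameter collection.
; It then checks its own Z: below zero it sets IsFlying and makes Flying the default land movement mode, otherwise it restores Walking.
; Only the default land mode is changed, with no direct SetMovementMode call.
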(event EventTick
  (params (DeltaSeconds :type Float%20%28single-precision%29))
  (bind _charactermovement (Variables|Character|GetCharacterMovement))
  (Rendering|Material|SetVectorParameterValue "/Game/Antares/Materials/SafeZone/MCP_PlayerPosition.MCP_PlayerPosition" "PlayerPosition" (Math|Conversions|ToLinearColor(Vector) (Transformation|GetActorLocation (Game|GetPlayerCharacter 0))) :!class /Script/Engine.KismetMaterialLibrary)
  (if (< (.z (Transformation|GetActorLocation)) 0.0)
    (Variables|Default|SetIsFlying true)
    (Variables|/Script/Engine.CharacterMovementComponent|SetDefaultLandMovementMode _charactermovement "MOVE_Flying")
    (else
      (Variables|Default|SetIsFlying false)
      (Variables|/Script/Engine.CharacterMovementComponent|SetDefaultLandMovementMode _charactermovement "MOVE_Walking"))))

(fn ConstructionScript)