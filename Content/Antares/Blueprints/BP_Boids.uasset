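; Niagara boids flock actor that reacts to the player and avoids the nearest nearby BP_SafeZone.
; Construction sizes the simulation grid, while Tick feeds avoidance and player location to Niagara.
; The outer sphere adjusts alignment and briefly pulls boids to center; the inner one targets the player unless safe-zoned.
; With the player in inner range, Niagara's particle export callback spawns BP_ForceField actors at a rotating subset of boid positions.
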(event OnComponentEndOverlap(OuterRange)
  (params (OverlappedComponent :type Primitive%20Component%20Object%20Reference) (OtherActor :type Actor%20Object%20Reference) (OtherComp :type Primitive%20Component%20Object%20Reference) (OtherBodyIndex :type Integer))
  (if (== OtherActor (Variables|Default|GetPlayer))
    (Niagara|SetNiagaraVariable(Float) (Variables|Default|GetNiagara) "AlignmentWeightIncrease" (Variables|Default|GetBaseGroupWeightIncrease))
    (Class|NiagaraComponent|SetVariableBool (Variables|Default|GetNiagara) "DestinationOverrideEnabled" false)))

(event OnComponentBeginOverlap(InnerRange)
  (params (OverlappedComponent :type Primitive%20Component%20Object%20Reference) (OtherActor :type Actor%20Object%20Reference) (OtherComp :type Primitive%20Component%20Object%20Reference) (OtherBodyIndex :type Integer) (bFromSweep :type Boolean) (SweepResult :type Hit%20Result%20Structure%20%28by%20ref%29))
  (bind _closestsafezone (Variables|Default|GetClosestSafeZone))
  (if (== OtherActor (Variables|Default|GetPlayer))
    (Variables|Default|SetPlayerInInnerRange true)
    (Utilities|IsValid _closestsafezone
      (:Is%20Valid
        (if (not (Variables|/Game/Antares/Blueprints/BP_SafeZone.BP_SafeZone_C|GetPlayerInside _closestsafezone))
          (Class|NiagaraComponent|SetVariableBool (Variables|Default|GetNiagara) "DestinationOverrideEnabled" true :!label _label)))
      (:Is%20Not%20Valid
        (goto _label)))))

(event OnComponentEndOverlap(InnerRange)
  (params (OverlappedComponent :type Primitive%20Component%20Object%20Reference) (OtherActor :type Actor%20Object%20Reference) (OtherComp :type Primitive%20Component%20Object%20Reference) (OtherBodyIndex :type Integer))
  (if (== OtherActor (Variables|Default|GetPlayer))
    (Variables|Default|SetPlayerInInnerRange false)
    (Class|NiagaraComponent|SetVariableBool (Variables|Default|GetNiagara) "DestinationOverrideEnabled" false)))

(event OnComponentBeginOverlap(OuterRange)
  (params (OverlappedComponent :type Primitive%20Component%20Object%20Reference) (OtherActor :type Actor%20Object%20Reference) (OtherComp :type Primitive%20Component%20Object%20Reference) (OtherBodyIndex :type Integer) (bFromSweep :type Boolean) (SweepResult :type Hit%20Result%20Structure%20%28by%20ref%29))
  (if (== OtherActor (Variables|Default|GetPlayer))
    (Niagara|SetNiagaraVariable(Float) (Variables|Default|GetNiagara) "AlignmentWeightIncrease" (Variables|Default|GetOuterRangeGroupWeightIncrease))
    (Class|NiagaraComponent|SetVariableBool (Variables|Default|GetNiagara) "DestinationOverrideEnabled" true)
    (Niagara|SetNiagaraVariable(Vector3) (Variables|Default|GetNiagara) "DestinationOverride" (Transformation|GetActorLocation))
    (Utilities|FlowControl|Delay 5.0)
    (if (not (Variables|Default|GetPlayerInInnerRange))
      (Class|NiagaraComponent|SetVariableBool (Variables|Default|GetNiagara) "DestinationOverrideEnabled" false))))

(event EventBeginPlay
  (Utilities|FlowControl|Sequence
    (:then_0
      (bind _outactors (Actor|GetAllActorsOfClass "/Game/Antares/Blueprints/BP_SafeZone.BP_SafeZone_C"))
      (Variables|Default|SetSafeZones _outactors))
    (:then_1
      (bind _returnvalue (Actor|GetActorOfClass "/Game/Antares/Blueprints/BP_TestCharacter.BP_TestCharacter_C"))
      (Variables|Default|SetPlayer _returnvalue))
    (:then_2
      (Class|NiagaraComponent|SetVariableObject (Variables|Default|GetNiagara) "User.BPCallback" self))))

(event EventParticleData
  (params (Data :type Array%20of%20Basic%20Particle%20Data%20Structures) (NiagaraSystem :type Niagara%20System%20Object%20Reference) (SimulationPositionOffset :type Vector%20%28by%20ref%29 :default "0, 0, 0"))
  (bind _particlecount (Variables|Default|GetParticleCount))
  (bind _returnvalue (/ _particlecount 2))
  (if (Variables|Default|GetPlayerInInnerRange)
    (for (_array_element _array_index) Data
      (if (== (Math|Integer|%(Integer) _array_index _returnvalue) (Variables|Default|GetIndex))
        (Game|SpawnActorfromClass "/Game/Antares/Blueprints/Chaos/BP_ForceField.BP_ForceField_C" (Math|Transform|MakeTransform (.Position (Utilities|Struct|BreakBasicParticleData _array_element)) "0, 0, 0" "1.500000,1.500000,1.500000") "Undefined" "MultiplyWithRoot" 0 0)))
    (bind _result (Math|Integer|IncrementInt (Variables|Default|GetIndex))
      (:%20%20
        (if (> _result (- _returnvalue 1))
          (Variables|Default|SetIndex 0))))))

(event EventTick
  (params (DeltaSeconds :type Float%20%28single-precision%29))
  (bind _niagara (Variables|Default|GetNiagara))
  (Utilities|FlowControl|Sequence
    (:then_0
      (Variables|Default|SetClosestSafeZoneDistance 9999999.0)
      (for _array_element (Variables|Default|GetSafeZones)
        (if (< (Math|Vector|VectorLengthSquared (- (Transformation|GetActorLocation _array_element) (Transformation|GetActorLocation))) (Variables|Default|GetClosestSafeZoneDistance))
          (Variables|Default|SetClosestSafeZoneDistance (Math|Vector|VectorLengthSquared (- (Transformation|GetActorLocation _array_element) (Transformation|GetActorLocation))))
          (Variables|Default|SetClosestSafeZone _array_element)))
      (Utilities|IsValid (Variables|Default|GetClosestSafeZone)
        (:Is%20Valid
          (Class|NiagaraComponent|SetVariableBool (Variables|Default|GetNiagara) "PointAvoidanceEnabled" true)
          (Niagara|SetNiagaraVariable(Vector3) (Variables|Default|GetNiagara) "PointAvoidanceLocation" (Transformation|GetActorLocation (Variables|Default|GetClosestSafeZone)))
          (Niagara|SetNiagaraVariable(Float) (Variables|Default|GetNiagara) "PointAvoidanceDistance" (+ (Variables|/Script/Engine.SphereComponent|GetSphereRadius (Variables|/Game/Antares/Blueprints/BP_SafeZone.BP_SafeZone_C|GetSafeZone (Variables|Default|GetClosestSafeZone))) (* (Variables|/Script/Engine.SphereComponent|GetSphereRadius (Variables|/Game/Antares/Blueprints/BP_SafeZone.BP_SafeZone_C|GetSafeZone (Variables|Default|GetClosestSafeZone))) 0.1)))
          (Niagara|SetNiagaraVariable(Float) (Variables|Default|GetNiagara) "PointAvoidanceDistanceDelta" (* (Variables|/Script/Engine.SphereComponent|GetSphereRadius (Variables|/Game/Antares/Blueprints/BP_SafeZone.BP_SafeZone_C|GetSafeZone (Variables|Default|GetClosestSafeZone))) 0.1)))
        (:Is%20Not%20Valid
          (Class|NiagaraComponent|SetVariableBool (Variables|Default|GetNiagara) "PointAvoidanceEnabled" false))))
    (:then_1
      (if (Variables|Default|GetPlayerInInnerRange)
        (Niagara|SetNiagaraVariable(Vector3) (Variables|Default|GetNiagara) "DestinationOverride" (Transformation|GetActorLocation (Variables|Default|GetPlayer)))))
    (:then_2
      (Utilities|IsValid (Variables|Default|GetClosestSafeZone)
        (:Is%20Valid
          (if (Variables|/Game/Antares/Blueprints/BP_SafeZone.BP_SafeZone_C|GetPlayerInside (Variables|Default|GetClosestSafeZone))
            (Utilities|FlowControl|Sequence
              (:then_0
                (Utilities|FlowControl|DoOnce false :!label _label
                  (:Completed
                    (Class|NiagaraComponent|SetVariableBool _niagara "DestinationOverrideEnabled" false))))
              (:then_1
                (goto _label_2 Reset)))
            (else
              (Utilities|FlowControl|Sequence
                (:then_0
                  (goto _label Reset))
                (:then_1
                  (Utilities|FlowControl|DoOnce false :!label _label_2
                    (:Completed
                      (if (Variables|Default|GetPlayerInInnerRange)
                        (Class|NiagaraComponent|SetVariableBool _niagara "DestinationOverrideEnabled" true)))))))))))
    (:then_3
      (if (Variables|Default|GetDrawDebug)
        (Rendering|Debug|DrawDebugBox (Transformation|GetActorLocation) (* (Variables|Default|GetGridSize) 0.5) "(R=0.000000,G=1.000000,B=0.000000,A=1.000000)" "0, 0, 0" 0.0 0.0)
        (Rendering|Debug|DrawDebugSphere (Transformation|GetActorLocation) (Components|Sphere|GetScaledSphereRadius (Variables|Default|GetOuterRange)) 12 "(R=1.000000,G=0.500000,B=0.000000,A=1.000000)" 0.0)
        (Rendering|Debug|DrawDebugSphere (Transformation|GetActorLocation) (Components|Sphere|GetScaledSphereRadius (Variables|Default|GetInnerRange)) 12 "(R=1.000000,G=0.000000,B=0.000000,A=1.000000)" 0.0)))))

(fn ConstructionScript
  (Niagara|SetNiagaraVariable(Vector3) (Variables|Default|GetNiagara) "GridSize" (Variables|Default|GetGridSize))
  (Class|NiagaraComponent|SetVariableInt (Variables|Default|GetNiagara) "CellsX" (Math|Float|Truncate (/ (.x (Variables|Default|GetGridSize)) 5e+01)))
  (Class|NiagaraComponent|SetVariableInt (Variables|Default|GetNiagara) "CellsY" (Math|Float|Truncate (/ (.y (Variables|Default|GetGridSize)) 5e+01)))
  (Class|NiagaraComponent|SetVariableInt (Variables|Default|GetNiagara) "CellsZ" (Math|Float|Truncate (/ (.z (Variables|Default|GetGridSize)) 5e+01)))
  (Class|NiagaraComponent|SetVariableInt (Variables|Default|GetNiagara) "ParticleCount" (Variables|Default|GetParticleCount))
  (Niagara|SetNiagaraVariable(Float) (Variables|Default|GetNiagara) "GroupWeightIncrease" (Variables|Default|GetBaseGroupWeightIncrease)))